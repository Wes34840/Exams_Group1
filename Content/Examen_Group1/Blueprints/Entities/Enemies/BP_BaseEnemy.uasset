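; Base enemy entity for action-based combat that picks its targets and signals when its action animation finishes.
; GetSmartTarget always returns "Attack" on a semi-random living player from GetRandomTarget.
; A per-player hit map spreads attacks by accepting random picks only near the least-hit count, seeding new players with the floored average.
; A separate GetRandomAction helper picks randomly among actions affordable with current mana, or "None".
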(event Custom|OnFinishedAnimation_event
  (params (Action :type Name))
  ;[0.15 0.15 0.15 0.5] Recall event to keep it similar to the player actions
  (Default|CallOnEnemyFinishedAction self))

(event EventBeginPlay
  ;[0.15 0.15 0.15 0.5] Recall event to keep it similar to the player actions
  (|CallParentFunction)
  (EventDispatchers|BindEventtoOnFinishedAction (delegate Custom|OnFinishedAnimation_event)))

(fn ConstructionScript
  (|CallParentFunction))

(fn GetSmartTarget
  (params (Entities :type Array%20of%20BP%20Base%20Entity%20Object%20References))
  ;[0.15 0.15 0.15 0.5] Override function
  (bind _entity (Targeting|GetRandomTarget Entities))
  (return "Attack" (Utilities|Array|MakeArray _entity)))

(fn GetEnemyName
  ;[0.15 0.15 0.15 0.5] GetEnemyName
  (return (Variables|Enemy|GetEnemyName)))

(fn GetRandomTarget
  (params (Entities :type Array%20of%20BP%20Base%20Entity%20Object%20References))
  (bind _l_validplayertargets (LocalVariables|GetL_ValidPlayerTargets))
  (bind _targetedentities (Variables|Default|GetTargetedEntities))
  ;[0.15 0.15 0.15 0.5] Gets the players that are alive
  (for _array_element Entities
    (if (CallFunction|CheckEntityHealthState _array_element)
      (Utilities|Array|Add (LocalVariables|GetL_ValidPlayerTargets) _array_element)))
  ;[0.15 0.15 0.15 0.5] Adds any new players to the attacked players map with the attack amount of the lowest attacked player
  (bind _values (Utilities|Map|Values (Variables|Default|GetTargetedEntities)))
  (for _array_element_2 (LocalVariables|GetL_ValidPlayerTargets)
    (if (not (Utilities|Map|Contains (Variables|Default|GetTargetedEntities) _array_element_2))
      (if (Utilities|Array|IsEmpty _values)
        (Utilities|Map|Add (Variables|Default|GetTargetedEntities) _array_element_2 0)
        (else
          (Utilities|Map|Add (Variables|Default|GetTargetedEntities) _array_element_2 (Math|Float|Floor (Math|Integer|AverageOfIntArray _values)))))))
  ;[0.15 0.15 0.15 0.5] Sorts what the most is that the enemy has hit players
  (for _array_element_3 (LocalVariables|GetL_ValidPlayerTargets)
    (Utilities|Array|Add (LocalVariables|GetL_SortedPlayerTargetHits) (.Value (Utilities|Map|Find (Variables|Default|GetTargetedEntities) _array_element_3))))
  (Class|KismetArrayLibrary|SortIntArray (LocalVariables|GetL_SortedPlayerTargetHits))
  ;[0.15 0.15 0.15 0.5] Gets a random player. If the player has been attacked more than twice the lowest attacked player, skip and get a different player
  (for _index (range 0 (Utilities|Array|Length _l_validplayertargets))
    (bind _output_get (LocalVariables|SetL_RandomEntity (.OutItem (Utilities|Array|Random _l_validplayertargets))))
    (if (< (.Value (Utilities|Map|Find (Variables|Default|GetTargetedEntities) _output_get)) (+ (Utilities|Array|Get(acopy) (LocalVariables|GetL_SortedPlayerTargetHits)) 2))
      (Utilities|Map|Add _targetedentities (LocalVariables|GetL_RandomEntity) (+ (.Value (Utilities|Map|Find _targetedentities (LocalVariables|GetL_RandomEntity))) 1))
      (return (LocalVariables|GetL_RandomEntity)))))

(fn GetRandomAction
  ;[0.15 0.15 0.15 0.5] Checks which actions of the ActionDataMap are valid and returns a random valid action
  (bind (_key _value) (Utilities|ForEachLoopMap (Variables|/Game/Examen_Group1/DataAssets/EntityActionData/PDA_ActionData_Base.PDA_ActionData_Base_C|GetActionData (CallFunction|GetActionDataMap)))
    (:Loop%20Body
      (if (> (Math|Float|Floor (Default|GetCurrentMana (Variables|Default|GetComp_Mana))) (.ManaCost (Utilities|Struct|BreakS_ActionData _value)))
        (Utilities|Map|Add (LocalVariables|GetL_ValidActions) _key _value)))
    (:Completed
      (if (Utilities|Map|IsEmpty (LocalVariables|GetL_ValidActions))
        (return "None")
        (else
          (bind _keys (Utilities|Map|Keys (LocalVariables|GetL_ValidActions)))
          (return (.OutItem (Utilities|Array|Random _keys))))))))