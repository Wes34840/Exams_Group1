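; BP_Boss is a child enemy Blueprint for a boss that chooses its attack and targets.
; GetSmartTarget rolls a random action, then returns all given entities as targets for AreaAttack or one random entity for any other action.
; Despite the function's name, selection is purely random, and the construction script only calls its parent.
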(fn ConstructionScript
  (|CallParentFunction))

(fn GetSmartTarget
  (params (Entities :type Array%20of%20BP%20Base%20Entity%20Object%20References))
  ;[0.15 0.15 0.15 0.5] Boss attacks
  (bind _chosenactionname (CallFunction|GetRandomAction))
  (if (== _chosenactionname "AreaAttack")
    (return _chosenactionname Entities)
    (else
      (bind _entity (CallFunction|GetRandomTarget Entities))
      (return _chosenactionname (Utilities|Array|MakeArray _entity)))))