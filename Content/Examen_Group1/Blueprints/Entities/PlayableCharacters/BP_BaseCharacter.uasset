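; Base playable character Blueprint that lets quick time event results scale incoming damage.
; Non-negative health changes pass straight to the parent's ApplyAction, while damaging effects are queued, as are reported QTE results.
; Whenever both queues have an entry, the oldest pair is consumed, applying damage multiplied by the Failed, Completed or Perfect factor.
; Completed and perfect results also trigger Block or PerfectBlock through Qte before resolution.
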(event EventCharacterCompletedQTE
  (params (Result :type E_QuickTimeEvent%20Enum :default "NewEnumerator0"))
  (bind _actioneffects (Variables|Default|GetActionEffects))
  (bind _output (Utilities|Array|Get(acopy) _actioneffects))
  (bind (_healthchange _statuseffects _self) (Utilities|Struct|BreakS_ActionEffect _output))
  (Utilities|Array|Add (Variables|Default|GetQuickTimeEvents) Result)
  (switch Utilities|FlowControl|Switch|SwitchonE_QuickTimeEvent Result
    (:NewEnumerator0
      _)
    (:NewEnumerator1
      (CallFunction|Qte "Block"))
    (:NewEnumerator2
      (CallFunction|Qte "PerfectBlock")))
  (if (and (Utilities|Array|IsValidIndex (Variables|Default|GetActionEffects)) (Utilities|Array|IsValidIndex (Variables|Default|GetQuickTimeEvents)))
    (CallFunction|SetTarget (Utilities|Array|MakeArray _self))
    (|CallParentFunction (Utilities|Struct|MakeS_ActionEffect (Math|Float|Round (* _healthchange (Utilities|Select :Index (Utilities|Array|Get(acopy) (Variables|Default|GetQuickTimeEvents)) :NewEnumerator0 (Variables|Default|GetFailed) :NewEnumerator1 (Variables|Default|GetCompleted) :NewEnumerator2 (Variables|Default|GetPerfect)))) _statuseffects _self))
    (Utilities|Array|RemoveIndex (Variables|Default|GetQuickTimeEvents))
    (Utilities|Array|RemoveIndex (Variables|Default|GetActionEffects))))

(event EventApplyAction
  (params (ActionEffect :type S%20Action%20Effect%20Structure))
  (bind _actioneffects (Variables|Default|GetActionEffects))
  (bind _output (Utilities|Array|Get(acopy) _actioneffects))
  (bind (_healthchange _statuseffects _self) (Utilities|Struct|BreakS_ActionEffect _output))
  (if (>= (Utilities|Struct|BreakS_ActionEffect ActionEffect) 0)
    (|CallParentFunction ActionEffect)
    (else
      (Utilities|Array|Add (Variables|Default|GetActionEffects) ActionEffect)
      (if (and (Utilities|Array|IsValidIndex (Variables|Default|GetActionEffects)) (Utilities|Array|IsValidIndex (Variables|Default|GetQuickTimeEvents)))
        (CallFunction|SetTarget (Utilities|Array|MakeArray _self))
        (|CallParentFunction (Utilities|Struct|MakeS_ActionEffect (Math|Float|Round (* _healthchange (Utilities|Select :Index (Utilities|Array|Get(acopy) (Variables|Default|GetQuickTimeEvents)) :NewEnumerator0 (Variables|Default|GetFailed) :NewEnumerator1 (Variables|Default|GetCompleted) :NewEnumerator2 (Variables|Default|GetPerfect)))) _statuseffects _self))
        (Utilities|Array|RemoveIndex (Variables|Default|GetQuickTimeEvents))
        (Utilities|Array|RemoveIndex (Variables|Default|GetActionEffects))))))

(fn ConstructionScript
  (|CallParentFunction))