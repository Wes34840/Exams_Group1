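; Networked player pawn that links a client's mobile UI to the character it owns and has perform actions.
; Client RPCs create and toggle the UI, while server RPCs display the selected or canceled action on a widget component and broadcast it through dispatchers.
; Class choice temporarily always spawns BP_RangedCharacter as the owned entity.
; The pawn forwards actions to that entity, relays its animation completion, and destroys it when itself destroyed.
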(event Custom|RPC_Server_UIAction_Canceled
  ;[0.15 0.15 0.15 0.5] Cancels the PlayerInput
  (Development|PrintText "UIEvent ActionInput Canceled")
  (CallFunction|DisplayInputonWidget "NewEnumerator0")
  (Default|CallOnUIActionCanceled (Variables|Identifier|GetPlayerID)))

(event Custom|RPC_Client_ToggleAttackUI
  (params (IsEnabled :type Boolean))
  ;[0.15 0.15 0.15 0.5] Disables the ability to return to the Attack UI
  (bind _mobileui (Variables|Refs|GetMobileUI)
    (:then
      (Default|ToggleAttackUI _mobileui IsEnabled))
    (:else)))

(event Custom|RPC_Client_InitUI
  (bind _returnvalue (Game|GetPlayerController 0))
  ;[0.15 0.15 0.15 0.5] Initiates the client's UI interface
  (bind _returnvalue_2 (UserInterface|CreateWidget "/Game/Examen_Group1/Widgets/WBP_MobileUI.WBP_MobileUI_C" _returnvalue))
  (bind _output_get (Variables|Refs|SetMobileUI _returnvalue_2))
  (UserInterface|Viewport|AddtoPlayerScreen _output_get)
  (Variables|/Script/Engine.PlayerController|SetbShowMouseCursor _returnvalue true)
  (Input|SetInputModeUIOnly _returnvalue (Variables|Refs|GetMobileUI) "DoNotLock" false)
  (Default|InitUI (Variables|Refs|GetMobileUI) self))

(event Custom|Server_NoneActionEvent
  ;[0.15 0.15 0.15 0.5] Error handling in the event the given UIAction is None
  (Development|PrintString "Error! None Selected as action!" true true "(R=1.000000,G=0.000000,B=0.000000,A=1.000000)" 15.0))

(event Custom|DisplayInputOnWidget
  (params (Input :type E_UIAction%20Enum :default "NewEnumerator0"))
  ;[0.15 0.15 0.15 0.5] Displays the input action of the player
  (Default|DisplayInput (Variables|Components|GetInputDisplayWidget) Input))

(event Custom|RPC_Server_UIAction_Selected
  (params (UIAction :type E_UIAction%20Enum :default "NewEnumerator0"))
  ;[0.15 0.15 0.15 0.5] Prints the text on the server stating the given UIEvent was called from which player
  (Development|PrintText (Utilities|Text|FormatText "UI Event on Player {PlayerID}: {Button}" (Variables|Identifier|GetPlayerID) (|GenerictoText UIAction)))
  (CallFunction|DisplayInputonWidget UIAction)
  (Default|CallOnUIActionSelected (Variables|Identifier|GetPlayerID) UIAction))

(event Custom|Client_UIEvent
  (params (Button :type E_UIAction%20Enum :default "NewEnumerator0"))
  ;[0.15 0.15 0.15 0.5] Prints the text of the pressed button on the client
  (Development|PrintText (Utilities|Text|FormatText "UI Event: {Button}" (|GenerictoText Button))))

(event Custom|Server_PerformActionOnEntity
  (params (Action :type E_UIAction%20Enum :default "NewEnumerator0") (ActionTarget :type BP%20Base%20Entity%20Object%20Reference%20%28by%20ref%29))
  ;[0.15 0.15 0.15 0.5] Performs the actions depending on the given parameter
  (if (Utilities|Enum|NotEqual(Enum) Action "NewEnumerator0")
    (Default|PerformAction (Variables|Refs|GetOwnedEntity) Action ActionTarget)
    (else
      (CallFunction|ServerNoneActionEvent))))

(event Custom|RPC_Server_ChooseClass
  ;[1 1 0 0.5] Temporary way the pawn spawns it's OwnedEntity (chosen class)
  (bind _returnvalue (Game|SpawnActorfromClass "/Game/Examen_Group1/Blueprints/Entities/PlayableCharacters/BP_RangedCharacter.BP_RangedCharacter_C" (Transformation|GetActorTransform) "Undefined" "MultiplyWithRoot" 0 "NewEnumerator0" 0))
  (bind _output_get (Variables|Refs|SetOwnedEntity _returnvalue))
  (EventDispatchers|BindEventtoOnFinishedAnimation _output_get (EventDispatchers|CreateEvent :!event Custom|OnEntityFinishedAnimation))
  (Default|CallOnClassChosen))

(event Custom|OnEntityFinishedAnimation
  ;[0.15 0.15 0.15 0.5] Calls the OnPawnCompletedAction dispatcher when the owned entity finishes it's animation
  (Default|CallOnPawnCompletedAction self))

(event EventBeginPlay
  ;[0.15 0.15 0.15 0.5] Gets a reference to the InputDisplay widget
  (bind _aswbp_player_input_display (Utilities|Casting|CastToWBP_PlayerInputDisplay (UserInterface|GetWidget (Variables|Default|GetServer_ChosenInput))))
  (Variables|Components|SetInputDisplayWidget _aswbp_player_input_display))

(event EventDestroyed
  ;[0.15 0.15 0.15 0.5] OnDestroyed, call a dispatcher that passes a self ref and get rid of the owned entity
  (Actor|DestroyActor (Variables|Refs|GetOwnedEntity))
  (Default|CallOnPawnDestroyed self))

(fn ConstructionScript)